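; Clickable door Blueprint that opens another level once the Keys, Coat and File flags are all set.
; On click it checks the flags in that order and, at the first one missing, passes that item's description text to the Message function.
; Message creates a description widget, adds it to the viewport and sets its text; the click graph removes it after a configurable delay.
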(event `self.ReceiveActorOnClicked`
  (params (ButtonPressed :type "Key Structure"))
  (`KismetSystemLibrary.PrintString` "door")
  (if (`self.keys`)
    (if (`self.coat`)
      (if (`self.file`)
        (`KismetSystemLibrary.PrintString` "Leaving")
        (`GameplayStatics.OpenLevel` (`self.Level`))
        (else
          (bind _widget (`self.Message` (`self.FileDesc`)))
          (`KismetSystemLibrary.Delay` (`self.Desc Persistance time`) :!label _label)
          (`Widget.RemoveFromParent` _widget)
          (`Widget.RemoveFromParent` (stale _widget_2))
          (`Widget.RemoveFromParent` (stale _widget_3))))
      (else
        (bind _widget_2 (`self.Message` (`self.coatDesc`)))
        (goto _label)))
    (else
      (bind _widget_3 (`self.Message` (`self.keysDesc`)))
      (goto _label))))

(fn `Message`
  (params (MesgText :type Text))
  (returns (Widget :type "/Game/Widgets/descriptionWidget Object Reference"))
  (bind _returnvalue (`|CreateWidget` "/Game/Widgets/descriptionWidget.descriptionWidget_C"))
  (`UserWidget.AddToViewport` _returnvalue 0)
  (bind _asdescription_widget (cast `/Game/Widgets/descriptionWidget` _returnvalue))
  (set `/Game/Widgets/descriptionWidget.DescText` MesgText _asdescription_widget)
  (return _returnvalue))

(fn `UserConstructionScript`)