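; Jacket pickup Blueprint that the player clicks to flag the coat as collected on a linked door.
; On click it prints a debug "Hello", casts its Door reference to Door_Blueprint and sets that door's Coat boolean to true.
; The jacket does not hide or destroy itself, and its other events are disabled stubs.
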(event `self.ReceiveActorOnClicked`
  (params (ButtonPressed :type "Key Structure"))
  (`KismetSystemLibrary.PrintString` "Hello")
  (bind _asdoor_blueprint (cast `/Game/bluePrints/Door_Blueprint` (`self.door`)))
  (set `/Game/bluePrints/Door_Blueprint.coat` true _asdoor_blueprint))

(fn `UserConstructionScript`
  (`parent.UserConstructionScript`))